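; FiringBox_BP is a shootable target that bobs vertically and awards score when damaged.
; Tick moves it along a sine wave around its spawn location, with a random time offset set at BeginPlay to vary the phase.
; On damage, the authority casts the instigator's PlayerState to MyPlayerState, then runs a ten-pass loop that increments score and destroys the box.
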(event `self.ReceiveBeginPlay`
  (set `self.self_loc` (`self.K2_GetActorLocation` self))
  (set `self.time_count` (`KismetMathLibrary.RandomFloatInRange` 0.0 (`self.T`))))

(event `self.ReceiveAnyDamage`
  (params (Damage :type "Float (single-precision)") (DamageType :type "DamageType Object Reference") (InstigatedBy :type "Controller Object Reference") (DamageCauser :type "Actor Object Reference"))
  (if (`KismetSystemLibrary.IsValid` InstigatedBy)
    (`/Engine/EditorBlueprintResources/ActorMacros.Switch Has Authority`
      (:`Authority`
        (bind _asmy_player_state (cast `/Game/Blueprints/MyPlayerState` (`Controller.PlayerState` InstigatedBy)))
        (for _ (range 10)
          (`/Game/Blueprints/MyPlayerState.IncrementScore` _asmy_player_state)
          (`self.K2_DestroyActor`))))))

(event `self.ReceiveTick`
  (params (DeltaSeconds :type "Float (single-precision)"))
  (bind (_self_loc_x _self_loc_y _self_loc_z) (`KismetMathLibrary.BreakVector` (`self.self_loc`)))
  (bind _output_get (set `self.time_count` (+ (`self.time_count`) DeltaSeconds)))
  (`self.K2_SetActorLocation` self (`KismetMathLibrary.MakeVector` _self_loc_x _self_loc_y (+ (* (`KismetMathLibrary.Sin` (`KismetMathLibrary.MultiplyByPi` (/ _output_get (`self.T`)))) 50.0) _self_loc_z)) false false))

(fn `UserConstructionScript`)